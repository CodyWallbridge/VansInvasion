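; Wave manager that runs endless rounds of enemy spawns with growing enemy counts.
; CountdownWave shows the Countdown widget and sets a timer for SpawnNextWave, which spawns random enemy types at reachable navmesh points around random AISpawnLocation actors.
; Each spawn is tracked and bound to its OnKilled event.
; EnemyKilled removes enemies from the list and, once it is empty, raises the next count and restarts the countdown.
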(event Custom|CountdownWave
  (bind _timeuntilwavebegins (Variables|Default|GetTimeUntilWaveBegins))
  (Variables|Default|GetW_Countdown
    (:then
      _)
    (:else
      (bind _returnvalue (UserInterface|CreateWidget "/Game/_Game/Countdown.Countdown_C" (Game|GetPlayerController 0)))
      (bind _output_get (Variables|Default|SetW_Countdown _returnvalue))
      (UserInterface|Viewport|AddtoViewport _output_get 0)))
  (Default|UpdateWaveTimer (Variables|Default|GetW_Countdown) _timeuntilwavebegins (Variables|Default|GetWave))
  (Utilities|Time|SetTimerbyFunctionName 0 "SpawnNextWave" (Math|Conversions|ToFloat(Integer) _timeuntilwavebegins))
  (Variables|Default|SetWave (+ (Variables|Default|GetWave) 1.0)))

(event Custom|SpawnNextWave
  (bind _outactors (Actor|GetAllActorsOfClass "/Game/_Game/AISpawnLocation.AISpawnLocation_C"))
  (Variables|Default|SetSpawners _outactors)
  (for _index (range 1 (Variables|Default|GetEnemiesToSpawn))
    (switch int (Math|Random|RandomIntegerinRange 0 5)
      (:Default
        (bind _returnvalue (Game|SpawnActorfromClass "/Game/_AI/enemies/Enemy_white.Enemy_white_C" (Math|Transform|MakeTransform (+ (.RandomLocation (AI|Navigation|GetRandomReachablePointinRadius (Transformation|GetActorLocation (Utilities|Array|Get(acopy) (Variables|Default|GetSpawners) (Math|Random|RandomIntegerinRange 0 (- (Utilities|Array|Length (Variables|Default|GetSpawners)) 1)))) 1e+03 0 0)) "0, 0,125.000000") "0, 0, 0" "1,1,1") "AdjustIfPossibleButAlwaysSpawn" 0 0))
        (CallFunction|EnemiesSpawned _returnvalue))
      (:0
        (bind _returnvalue_2 (Game|SpawnActorfromClass "/Game/_AI/enemies/Enemy_big.Enemy_big_C" (Math|Transform|MakeTransform (+ (.RandomLocation (AI|Navigation|GetRandomReachablePointinRadius (Transformation|GetActorLocation (Utilities|Array|Get(acopy) (Variables|Default|GetSpawners) (Math|Random|RandomIntegerinRange 0 (- (Utilities|Array|Length (Variables|Default|GetSpawners)) 1)))) 1e+03 0 0)) "0, 0,125.000000") "0, 0, 0" "1,1,1") "AdjustIfPossibleButAlwaysSpawn" 0 0))
        (CallFunction|EnemiesSpawned _returnvalue_2))
      (:1
        (bind _returnvalue_3 (Game|SpawnActorfromClass "/Game/_AI/enemies/EnemY_bigblueglow.EnemY_bigblueglow_C" (Math|Transform|MakeTransform (+ (.RandomLocation (AI|Navigation|GetRandomReachablePointinRadius (Transformation|GetActorLocation (Utilities|Array|Get(acopy) (Variables|Default|GetSpawners) (Math|Random|RandomIntegerinRange 0 (- (Utilities|Array|Length (Variables|Default|GetSpawners)) 1)))) 1e+03 0 0)) "0, 0,125.000000") "0, 0, 0" "1,1,1") "AdjustIfPossibleButAlwaysSpawn" 0 0))
        (CallFunction|EnemiesSpawned _returnvalue_3))
      (:2
        (bind _returnvalue_4 (Game|SpawnActorfromClass "/Game/_AI/enemies/Enemy_forest.Enemy_forest_C" (Math|Transform|MakeTransform (+ (.RandomLocation (AI|Navigation|GetRandomReachablePointinRadius (Transformation|GetActorLocation (Utilities|Array|Get(acopy) (Variables|Default|GetSpawners) (Math|Random|RandomIntegerinRange 0 (- (Utilities|Array|Length (Variables|Default|GetSpawners)) 1)))) 1e+03 0 0)) "0, 0,125.000000") "0, 0, 0" "1,1,1") "AdjustIfPossibleButAlwaysSpawn" 0 0))
        (CallFunction|EnemiesSpawned _returnvalue_4))
      (:3
        (bind _returnvalue_5 (Game|SpawnActorfromClass "/Game/_AI/enemies/Enemy_blueglow.Enemy_blueglow_C" (Math|Transform|MakeTransform (+ (.RandomLocation (AI|Navigation|GetRandomReachablePointinRadius (Transformation|GetActorLocation (Utilities|Array|Get(acopy) (Variables|Default|GetSpawners) (Math|Random|RandomIntegerinRange 0 (- (Utilities|Array|Length (Variables|Default|GetSpawners)) 1)))) 1e+03 0 0)) "0, 0,125.000000") "0, 0, 0" "1,1,1") "AdjustIfPossibleButAlwaysSpawn" 0 0))
        (CallFunction|EnemiesSpawned _returnvalue_5))
      (:4
        (bind _returnvalue_6 (Game|SpawnActorfromClass "/Game/_AI/enemies/Enemy_lava.Enemy_lava_C" (Math|Transform|MakeTransform (+ (.RandomLocation (AI|Navigation|GetRandomReachablePointinRadius (Transformation|GetActorLocation (Utilities|Array|Get(acopy) (Variables|Default|GetSpawners) (Math|Random|RandomIntegerinRange 0 (- (Utilities|Array|Length (Variables|Default|GetSpawners)) 1)))) 1e+03 0 0)) "0, 0,125.000000") "0, 0, 0" "1,1,1") "AdjustIfPossibleButAlwaysSpawn" 0 0))
        (CallFunction|EnemiesSpawned _returnvalue_6)))))

(event EventBeginPlay
  (Utilities|FlowControl|Sequence
    (:then_0
      (Utilities|FlowControl|Delay 0.2)
      (bind _outactors (Actor|GetAllActorsOfClass "/Game/_Game/AISpawnLocation.AISpawnLocation_C"))
      (for _array_element _outactors
        (Utilities|Array|Add (Variables|Default|GetSpawners) _array_element)))
    (:then_1
      (Utilities|FlowControl|Delay 2.0)
      (CallFunction|CountdownWave))))

(fn ConstructionScript)

(fn EnemyKilled
  (params (Enemy :type BP%20Enemy%20Base%20Object%20Reference))
  (bind _enemies (Variables|Default|GetEnemies))
  (Utilities|Array|RemoveItem _enemies Enemy)
  (if (<= (Utilities|Array|Length _enemies) 0)
    (Variables|Default|SetEnemiesToSpawn (+ (Variables|Default|GetEnemiesToSpawn) (Math|Random|RandomIntegerinRange 2 3)))
    (CallFunction|CountdownWave)))

(fn EnemiesSpawned
  (params (Enemy :type BP%20Enemy%20Base%20Object%20Reference))
  (Utilities|Array|Add (Variables|Default|GetEnemies) Enemy)
  (EventDispatchers|BindEventtoOnKilled Enemy (EventDispatchers|CreateEvent :!event EnemyKilled)))