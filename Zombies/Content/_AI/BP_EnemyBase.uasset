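; Base enemy character that chases a target, attacks it in melee and can drop a pickup on death.
; ChasePlayer moves via AIMoveTo, then Att plays a montage whose notify runs a sphere overlap to damage ThirdPersonCharacters before chasing again.
; BeginPlay pre-rolls an occasional health, coin or defence drop.
; Death fires OnKilled, disables movement and collision, and spawns that drop; a separate event adds Score to the player.
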(event Custom|ChasePlayer
  (params (Target :type Pawn%20Object%20Reference))
  ;[1 1 1] chase and death
  (bind _output_get (Variables|Default|SetPlayer%20Target Target))
  (AI|AIMoveTo self "0, 0, 0" _output_get 5.0 false
    (:OnSuccess
      (CallFunction|Att))))

(event Custom|Att
  ;[1 1 1] attack
  (Animation|Montage|PlayMontage (Variables|Character|GetMesh) (Variables|Default|GetMontage%20to%20Play%20Hitting)
    (:OnNotifyBegin
      (bind (_outactors _returnvalue) (Collision|SphereOverlapActors (Transformation|GetWorldLocation (Variables|Default|GetAttack%20Point)) 6e+01 (Utilities|Array|MakeArray "ObjectTypeQuery3") "/Game/ThirdPersonBP/Blueprints/ThirdPersonCharacter.ThirdPersonCharacter_C"))
      (if _returnvalue
        (for _array_element _outactors
          (Game|Damage|ApplyDamage _array_element (Variables|Default|GetDamage) 0 self "/Script/Engine.DamageType"))
        (Utilities|FlowControl|Delay 1.0)
        (CallFunction|ChasePlayer (Variables|Default|GetPlayer%20Target))
        (else
          (CallFunction|ChasePlayer (Variables|Default|GetPlayer%20Target)))))))

(event Custom|Death
  (bind _returnvalue (Transformation|GetActorLocation))
  (bind _returnvalue_2 (* _returnvalue "1.000000,1.000000, 0"))
  ;[1 1 1] chase and death
  (if (not (Variables|Default|GetDead))
    (Variables|Default|SetDead true)
    (Default|CallOnKilled self)
    (Pawn|Components|CharacterMovement|DisableMovement (Variables|Character|GetCharacterMovement))
    (Collision|SetCollisionEnabled (Variables|Collision|GetCapsuleComponent) "NoCollision")
    (AI|Navigation|StopMovement (Pawn|GetController))
    (if (Variables|Default|GethasDrop)
      (switch int (Variables|Default|GetdropType)
        (:Default
          (Game|SpawnActorfromClass "/Game/_AI/pickups/SM_Pickup_Defence_2.SM_Pickup_Defence_2_C" (Math|Transform|MakeTransform (+ _returnvalue_2 "0, 0,120.000000") "0, 0, 0" "2.000000,2.000000,2.000000") "AdjustIfPossibleButAlwaysSpawn" 0 0))
        (:0
          (Game|SpawnActorfromClass "/Game/_AI/pickups/SM_Pickup_Health.SM_Pickup_Health_C" (Math|Transform|MakeTransform (+ _returnvalue_2 "0, 0,50.000000") "0, 0, 0" "2.000000,2.000000,2.000000") "AdjustIfPossibleButAlwaysSpawn" 0 0))
        (:1
          (Game|SpawnActorfromClass "/Game/_AI/pickups/SM_Coin_1.SM_Coin_1_C" (Math|Transform|MakeTransform (+ _returnvalue_2 "0, 0,100.000000") "0, 0, 0" "10.000000,10.000000,10.000000") "AdjustIfPossibleButAlwaysSpawn" 0 0))))))

(event Custom|UpdatePlayerScore
  ;[1 1 1] chase and death
  (bind _asthird_person_character (Utilities|Casting|CastToThirdPersonCharacter (Game|GetPlayerCharacter 0)))
  (Default|UpdateScore _asthird_person_character (Variables|Default|GetScore)))

(event EventBeginPlay
  ;[1 1 1] startup Delay
  (if (<= (Math|Random|RandomIntegerinRange 0 100) 20)
    (Variables|Default|SethasDrop true)
    (Variables|Default|SetdropType (Math|Random|RandomIntegerinRange 0 2))))

(fn ConstructionScript)